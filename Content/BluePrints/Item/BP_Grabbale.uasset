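; BP_Grabbale is an item actor that the player can pick up and drop.
; Interact, when the player holds nothing, disables the root's physics and collision, hands the item to BP_Player's Grab, then scales up a Niagara effect after a short delay.
; Drop detaches it in world space, restores collision and physics, and hides the effect.
; An overlap box shows a WBP_UI01 how-to-use widget while the player is inside.
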(event OnComponentBeginOverlap(UIBox)
  (params (OverlappedComponent :type Primitive%20Component%20Object%20Reference) (OtherActor :type Actor%20Object%20Reference) (OtherComp :type Primitive%20Component%20Object%20Reference) (OtherBodyIndex :type Integer) (bFromSweep :type Boolean) (SweepResult :type Hit%20Result%20Structure%20%28by%20ref%29))
  ;[0.15 0.15 0.15 0.5] UI
  (if (== OtherActor (Variables|Default|GetAs%20BP%20Player))
    (Utilities|GetDataTableRow "/Game/BluePrints/Datas/DataTable/SOP/DTHowtouse.DTHowtouse" "1"
      (:then
        (bind _returnvalue (UserInterface|CreateWidget "/Game/UI/WBP_UI01.WBP_UI01_C" 0 "1"))
        (bind _output_get (Variables|Default|SetHUD _returnvalue))
        (UserInterface|Viewport|AddtoViewport _output_get 0)))))

(event OnComponentEndOverlap(UIBox)
  (params (OverlappedComponent :type Primitive%20Component%20Object%20Reference) (OtherActor :type Actor%20Object%20Reference) (OtherComp :type Primitive%20Component%20Object%20Reference) (OtherBodyIndex :type Integer))
  ;[0.15 0.15 0.15 0.5] UI
  (if (== OtherActor (Variables|Default|GetAs%20BP%20Player))
    (bind _output_get (Variables|Default|SetHUD (Variables|Default|GetHUD)))
    (Utilities|IsValid _output_get
      (:Is%20Valid
        (Widget|RemovefromParent (Variables|Default|GetHUD))))))

(event Custom|Drop
  ;[0.15 0.15 0.15 0.5] 물건 놓기
  (Collision|SetActorEnableCollision true)
  (Transformation|DetachFromActor "KeepWorld" "KeepWorld" "KeepWorld")
  (Collision|SetCollisionEnabled (Variables|Default|GetRoot) "QueryAndPhysics")
  (Transformation|SetRelativeScale3D (Variables|Default|GetNiagara) "0, 0, 0")
  (Physics|SetSimulatePhysics (Variables|Default|GetRoot) true))

(event EventBeginPlay
  (bind _asbp_player (Utilities|Casting|CastToBP_Player (Game|GetPlayerCharacter 0)))
  (Variables|Default|SetAs%20BP%20Player _asbp_player))

(event Collision|EventActorBeginOverlap
  (params (OtherActor :type Actor%20Object%20Reference)))

(event EventTick
  (params (DeltaSeconds :type Float%20%28single-precision%29)))

(event EventInteract
  (params (Player :type BP%20Player%20Object%20Reference))
  (if (not (.ReturnValue (Default|GetGrabbedObject Player)))
    (Physics|SetSimulatePhysics (Variables|Default|GetRoot) false)
    (Collision|SetCollisionEnabled (Variables|Default|GetRoot) "NoCollision")
    (Default|Grab Player self)
    (Utilities|FlowControl|Delay 0.3)
    (Transformation|SetRelativeScale3D (Variables|Default|GetNiagara) "0.010000,0.010000,0.010000")))

(fn ConstructionScript)