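; BP_Elevator is an elevator item actor that shows a how-to-use prompt while the player stands in its trigger box.
; On overlap with the cached player reference, it looks up row "2" in DTHowtouse and, if found, adds a WBP_UI01 widget for that row to the viewport.
; Ending the overlap removes the widget.
; The graphs here contain no elevator movement logic.
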(event OnComponentBeginOverlap(Box_0)
  (params (OverlappedComponent :type Primitive%20Component%20Object%20Reference) (OtherActor :type Actor%20Object%20Reference) (OtherComp :type Primitive%20Component%20Object%20Reference) (OtherBodyIndex :type Integer) (bFromSweep :type Boolean) (SweepResult :type Hit%20Result%20Structure%20%28by%20ref%29))
  (if (== OtherActor (Variables|Default|GetAs%20BP%20Player))
    (Utilities|GetDataTableRow "/Game/BluePrints/Datas/DataTable/SOP/DTHowtouse.DTHowtouse" "2"
      (:then
        (bind _returnvalue (UserInterface|CreateWidget "/Game/UI/WBP_UI01.WBP_UI01_C" 0 "2"))
        (bind _output_get (Variables|Default|SetHUD_0 _returnvalue))
        (UserInterface|Viewport|AddtoViewport _output_get 0)))))

(event OnComponentEndOverlap(Box_0)
  (params (OverlappedComponent :type Primitive%20Component%20Object%20Reference) (OtherActor :type Actor%20Object%20Reference) (OtherComp :type Primitive%20Component%20Object%20Reference) (OtherBodyIndex :type Integer))
  (if (== OtherActor (Variables|Default|GetAs%20BP%20Player))
    (bind _output_get (Variables|Default|SetHUD_0 (Variables|Default|GetHUD_0)))
    (Utilities|IsValid _output_get
      (:Is%20Valid
        (Widget|RemovefromParent (Variables|Default|GetHUD_0))))))

(event EventBeginPlay
  (|CallParentFunction))

(event Collision|EventActorBeginOverlap
  (params (OtherActor :type Actor%20Object%20Reference))
  (|CallParentFunction OtherActor) ; This node is disabled and will not be called.\nDrag off pins to build functionality.
)

(event EventTick
  (params (DeltaSeconds :type Float%20%28single-precision%29))
  (|CallParentFunction DeltaSeconds) ; This node is disabled and will not be called.\nDrag off pins to build functionality.
)

(fn ConstructionScript
  (|CallParentFunction))