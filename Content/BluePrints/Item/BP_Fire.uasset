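; BP_Fire is a fire actor that tags overlapping actors as Burning, sends them BurnMessage, and spreads by spawning copies of itself.
; A timer picks unused random directions, sphere-traces to skip spots with Burning actors, and spawns children with SpreadPower one lower to limit propagation.
; ReducePower halts timers, updates the progress-bar widget, then destroys the fire at zero or schedules restoration.
; RestorePower refills Power through a timeline started from the current level.
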(event OnComponentBeginOverlap(Box)
  (params (OverlappedComponent :type Primitive%20Component%20Object%20Reference) (OtherActor :type Actor%20Object%20Reference) (OtherComp :type Primitive%20Component%20Object%20Reference) (OtherBodyIndex :type Integer) (bFromSweep :type Boolean) (SweepResult :type Hit%20Result%20Structure%20%28by%20ref%29))
  (Utilities|Array|Add (Variables|/Script/Engine.Actor|GetTags OtherActor) (CallFunction|GetTagsLibrary "(TagName=\"Burning\")"))
  (Class|BPBurn|Burn(Message) OtherActor self))

(event OnComponentEndOverlap(Box)
  (params (OverlappedComponent :type Primitive%20Component%20Object%20Reference) (OtherActor :type Actor%20Object%20Reference) (OtherComp :type Primitive%20Component%20Object%20Reference) (OtherBodyIndex :type Integer))
  (Utilities|Array|RemoveItem (Variables|/Script/Engine.Actor|GetTags OtherActor) (CallFunction|GetTagsLibrary "(TagName=\"Burning\")")))

(event Custom|OnSpreadTimerFinish
  (CallFunction|Spread)
  (if (CallFunction|CanSpread)
    (Utilities|StartSpreadingTimer)))

(event Custom|ReducePower
  (params (PowertoReduce :type Float%20%28double-precision%29))
  ;[0.15 0.15 0.15 0.5] 파워 줄이기
  (Utilities|StopTimers)
  (Utilities|FlowControl|Sequence
    (:then_0
      ;[0.15 0.15 0.15 0.5] ui
      (Utilities|Update (- (Variables|Default|Getpower) PowertoReduce)))
    (:then_1
      (if (> (Variables|Default|Getpower) 0.0)
        ;[0.15 0.15 0.15 0.5] 타이머를 복구
        (bind _returnvalue (Utilities|Time|SetTimerbyEvent (EventDispatchers|CreateEvent :!event Custom|RestorePower) (Variables|Default|GetTimetoStartRestore)))
        (Variables|Default|SetRestoreTimer _returnvalue)
        (else
          (Actor|DestroyActor))))))

(event Custom|RestorePower
  (bind _tl_restorefire (Variables|Default|GetTL_RestoreFire))
  ;[0.15 0.15 0.15 0.5] 에너지(Power) 바를 다시 가득 채우기
  (Components|Timeline|SetNewTime _tl_restorefire (* (Variables|Default|Getpower) (Components|Timeline|GetTimelineLength _tl_restorefire)))
  (bind _alpha (Timeline|TL_RestoreFire Play)
    (:Update
      (Utilities|Update _alpha)
      (if (Math|Conversions|ToBoolean(Integer) (Variables|Default|GetSpreadPower))
        (Utilities|StartSpreadingTimer)))))

(event EventBeginPlay
  (if (Math|Conversions|ToBoolean(Integer) (Variables|Default|GetSpreadPower))
    (Utilities|StartSpreadingTimer)))

(fn ConstructionScript)

(fn Spread
  (bind _returnvalue (Transformation|GetActorLocation))
  (if (CallFunction|CanSpread)
    (Utilities|FlowControl|Sequence
      (:then_0
        ;[0.15 0.15 0.15 0.5] 스폰 로케이션 찾기
        ;;[0.15 0.15 0.15 0.5] 중복 방지
        (if true
          (bind _outitem (Utilities|Array|Random (Variables|Default|GetDirections) :!label _label))
          (if (Utilities|Array|ContainsItem (Variables|Default|GetUsedDirections) _outitem)
            (goto _label)
            (else
              (Utilities|Array|Add (Variables|Default|GetUsedDirections) _outitem)
              (LocalVariables|SetSpawnLocation (+ (* _outitem (Variables|Default|GetSpreadDistance)) (Math|Vector|MakeVector (.x _returnvalue) (.y _returnvalue) 0.0)))))))
      (:then_1
        (if (CallFunction|CanSpawn (LocalVariables|GetSpawnLocation))
          (Game|SpawnActorfromClass "BP_Fire_C" (Math|Transform|MakeTransform (LocalVariables|GetSpawnLocation) "0, 0, 0" "1.000000,1.000000,1.000000") "Undefined" "MultiplyWithRoot" 0 (- (Variables|Default|GetSpreadPower) 1) 0)
          (else
            (CallFunction|Spread)))))))

(fn CanSpawn
  (params (SpawnLocation :type Vector))
  (bind (_x _y _z) (Math|Vector|BreakVector SpawnLocation))
  (bind (_outhits _returnvalue) (Collision|MultiSphereTraceByChannel SpawnLocation (Math|Vector|MakeVector _x _y (+ _z 1e+02)) 3e+01 "TraceTypeQuery1" false 0 "ForDuration"))
  (if _returnvalue
    (for _array_element _outhits
      (if (Actor|ActorHasTag (.HitActor (Collision|BreakHitResult _array_element)) (Utilities|Name|MakeLiteralName "Burning"))
        (return false)))
    (return true)
    (else
      (return true))))

(fn CanSpread
  (return (!= (Utilities|Array|Length (Variables|Default|GetUsedDirections)) (Utilities|Array|Length (Variables|Default|GetDirections)))))