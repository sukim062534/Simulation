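; BP_Box01 is a flammable box that catches fire and spreads it to other BP_Box01 actors through overlaps.
; Ignit enables the spread Sphere, drops repeating burn decals and scales up fire particles, then chains timelines through Burning's red overlay material into Extingish, which rescales the particles.
; A burning box ignites boxes touching its Box or entering its Sphere.
; The logic resetting IsitBurning is disconnected, so it stays true.
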(event OnComponentBeginOverlap(Box)
  (params (OverlappedComponent :type Primitive%20Component%20Object%20Reference) (OtherActor :type Actor%20Object%20Reference) (OtherComp :type Primitive%20Component%20Object%20Reference) (OtherBodyIndex :type Integer) (bFromSweep :type Boolean) (SweepResult :type Hit%20Result%20Structure%20%28by%20ref%29))
  ;[0.15 0.15 0.15 0.5] Comment
  (bind _output_get (Variables|Default|SetOther%20Actor OtherActor))
  (if (not (== _output_get self))
    (bind _asbp_box_01 (Utilities|Casting|CastToBP_Box01 (Variables|Default|GetOther%20Actor)))
    (if (Variables|BP_Box01_C|GetisitBurning _asbp_box_01)
      (if (not (Variables|Default|GetisitBurning))
        (CallFunction|Ignit)))))

(event OnComponentBeginOverlap(Sphere)
  (params (OverlappedComponent :type Primitive%20Component%20Object%20Reference) (OtherActor :type Actor%20Object%20Reference) (OtherComp :type Primitive%20Component%20Object%20Reference) (OtherBodyIndex :type Integer) (bFromSweep :type Boolean) (SweepResult :type Hit%20Result%20Structure%20%28by%20ref%29))
  ;[0.15 0.15 0.15 0.5] Comment
  (bind _output_get (Variables|Default|SetOther%20Actor OtherActor))
  (if (not (== _output_get self))
    (bind _asbp_box_01 (Utilities|Casting|CastToBP_Box01 (Variables|Default|GetOther%20Actor)))
    (if (not (Variables|BP_Box01_C|GetisitBurning _asbp_box_01))
      (CallFunction|Ignit _asbp_box_01))))

(event Custom|CreateDecal
  ;[0.15 0.15 0.15 0.5] 그을린 자국
  (if (not (Variables|Default|GetDecalExtingish)) :!label _label
    (Rendering|Decal|SpawnDecalatLocation "/Game/BluePrints/Item/Material/Burnt_Mat.Burnt_Mat" "60.000000,60.000000,60.000000" (Transformation|GetWorldLocation (Variables|Default|GetBox)) "-90.000000,0.000000,0.000000" 0.0)
    (Utilities|FlowControl|Delay 0.5)
    (goto _label)))

(event Custom|Burning
  ;[0.15 0.15 0.15 0.5] 색상 변경
  (Variables|Default|SetisitBurning true)
  (CallFunction|Red)
  (bind _alpha (Timeline|Timeline_5 Play)
    (:Update
      (Rendering|Material|SetVectorParameterValue (Variables|Default|GetOverlay) "Opacity" (Math|Conversions|ToLinearColor(Float) _alpha) :!class /Script/Engine.MaterialInstanceDynamic))
    (:Finished
      (CallFunction|Extingish))))

(event Custom|Ignit
  ;[0.15 0.15 0.15 0.5] Comment
  (Collision|SetCollisionEnabled (Variables|Default|GetSphere) "QueryAndProbe")
  (if (not (Variables|Default|GetDecalExtingish))
    (CallFunction|CreateDecal)
    (bind _alpha (Timeline|Timeline_4 Play)
      (:Update
        (Transformation|SetRelativeScale3D (Variables|Default|GetParticleSystem) (Math|Conversions|ToVector(Float) _alpha)))
      (:Finished
        (CallFunction|Burning)))))

(event Custom|Extingish
  ;[0.15 0.15 0.15 0.5] 그을린 자국
  (Rendering|Material|SetVectorParameterValue (Variables|Default|GetOverlay) "Color" (stale _newtrack_2) :!class /Script/Engine.MaterialInstanceDynamic)
  (bind _alpha (Timeline|Timeline_7 Play)
    (:Update
      (Transformation|SetRelativeScale3D (Variables|Default|GetParticleSystem) (Math|Conversions|ToVector(Float) _alpha)))))

(event EventBeginPlay
  (Collision|SetCollisionEnabled (Variables|Default|GetSphere) "NoCollision"))

(fn ConstructionScript)

(fn Red
  (bind _returnvalue (Rendering|Material|CreateDynamicMaterialInstance "/Game/BluePrints/Item/Material/M_Box01.M_Box01" "None" "None" :!class /Script/Engine.KismetMaterialLibrary))
  (bind _output_get (Variables|Default|SetOverlay _returnvalue))
  (Rendering|Material|SetOverlayMaterial (Variables|Default|GetStaticMesh) _output_get :!class /Script/Engine.MeshComponent)
  (Rendering|Material|SetScalarParameterValue (Variables|Default|GetOverlay) "Opacity" 0.0 :!class /Script/Engine.MaterialInstanceDynamic)
  (Rendering|Material|SetVectorParameterValue (Variables|Default|GetOverlay) "Color" "(R=1.000000,G=0.021327,B=0.000000,A=1.000000)" :!class /Script/Engine.MaterialInstanceDynamic))