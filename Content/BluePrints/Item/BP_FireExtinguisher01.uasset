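; Fire extinguisher world item that reacts when the player comes within range of it.
; Player overlap with UIBox fires begin/end dispatchers and toggles a custom-depth outline on the mesh.
; Entering also looks up row "2" of DTHowtouse and, if found, shows a BP_UI01 widget, which is removed on exit.
; Init functions set the item's ID, type, name, UI prefix and static mesh.
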(event OnComponentBeginOverlap(UIBox)
  (params (OverlappedComponent :type Primitive%20Component%20Object%20Reference) (OtherActor :type Actor%20Object%20Reference) (OtherComp :type Primitive%20Component%20Object%20Reference) (OtherBodyIndex :type Integer) (bFromSweep :type Boolean) (SweepResult :type Hit%20Result%20Structure%20%28by%20ref%29))
  (Utilities|FlowControl|Sequence
    (:then_0
      (if (== OtherActor (Variables|Default|GetAs%20BP%20Player))
        (Default|CallOnBeginOverlap self)
        (CallFunction|EnableOutLine true)
        (Utilities|GetDataTableRow "/Game/BluePrints/Datas/DataTable/SOP/DTHowtouse.DTHowtouse" "2"
          (:then
            (bind _returnvalue (UserInterface|CreateWidget "/Game/UI/BP_UI01.BP_UI01_C"))
            (bind _output_get (Variables|Default|SetHUD _returnvalue))
            (UserInterface|Viewport|AddtoViewport _output_get 0)))))))

(event OnComponentEndOverlap(UIBox)
  (params (OverlappedComponent :type Primitive%20Component%20Object%20Reference) (OtherActor :type Actor%20Object%20Reference) (OtherComp :type Primitive%20Component%20Object%20Reference) (OtherBodyIndex :type Integer))
  (if (== OtherActor (Variables|Default|GetAs%20BP%20Player))
    (Default|CallOnEndOverlap self)
    (CallFunction|EnableOutLine false)
    (bind _output_get (Variables|Default|SetHUD (Variables|Default|GetHUD)))
    (Utilities|IsValid _output_get
      (:Is%20Valid
        (Widget|RemovefromParent (Variables|Default|GetHUD))))))

(event EventBeginPlay
  (|CallParentFunction))

(event Collision|EventActorBeginOverlap
  (params (OtherActor :type Actor%20Object%20Reference))
  (|CallParentFunction OtherActor))

(event EventTick
  (params (DeltaSeconds :type Float%20%28single-precision%29))
  (|CallParentFunction DeltaSeconds))

(fn ConstructionScript
  (|CallParentFunction))

(fn InitSpawnData
  (params (ID :type Name))
  (Variables|Default|SetID ID))

(fn InitWorldItemBaseData
  (params (ItemType :type E_ItemType%20Enum :default "NewEnumerator0") (ItemName :type Text) (UIPreFix :type E_UIPrefix%20Enum :default "NewEnumerator0") (StaticMesh :type Static%20Mesh%20Object%20Reference))
  (Variables|Default|SetItemType ItemType)
  (Variables|Default|SetItemName ItemName)
  (Variables|Default|SetUIPrefix UIPreFix)
  (Components|StaticMesh|SetStaticMesh (Variables|Default|GetStaticMesh) StaticMesh))

(fn EnableOutLine
  (params (bIsEnabled :type Boolean))
  (Rendering|SetRenderCustomDepth (Variables|Default|GetStaticMesh) bIsEnabled))